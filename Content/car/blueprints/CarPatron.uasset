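; Player-drivable car Blueprint built on Chaos wheeled vehicle movement.
; Throttle, brake, steering and handbrake inputs feed straight into the vehicle movement component.
; Each tick it reads the first wheel's steer angle and applies it, negated, as pitch on the Wheel component, apparently a steering wheel, with fixed yaw.
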(event EventTick
  (params (DeltaSeconds :type Float%20%28single-precision%29))
  (bind _aschaos_wheeled_vehicle_movement_component (Utilities|Casting|CastToChaosWheeledVehicleMovementComponent (Variables|Default|GetVehicleMovementComponent)))
  (Variables|Default|SetSteerAngle (Class|ChaosVehicleWheel|GetSteerAngle (Utilities|Array|Get(acopy) (Variables|/Script/ChaosVehicles.ChaosWheeledVehicleMovementComponent|GetWheels _aschaos_wheeled_vehicle_movement_component))))
  (Transformation|SetRelativeRotation (Variables|Default|Getwheel) (Math|Rotator|MakeRotator 0.0 (* (Class|ChaosVehicleWheel|GetSteerAngle (Utilities|Array|Get(acopy) (Variables|/Script/ChaosVehicles.ChaosWheeledVehicleMovementComponent|GetWheels _aschaos_wheeled_vehicle_movement_component))) -1.0) 9e+01) false false))

(event Input|ActionEvents|InputActionHandBrake
  (params (Key :type Key%20Structure))
  (bind _vehiclemovementcomponent (Variables|Default|GetVehicleMovementComponent))
  (:Pressed
    (Class|ChaosVehicleMovementComponent|SetHandbrakeInput _vehiclemovementcomponent true))
  (:Released
    (Class|ChaosVehicleMovementComponent|SetHandbrakeInput _vehiclemovementcomponent false)))

(event Input|AxisEvents|InputAxisThrottel
  (params (AxisValue :type Float%20%28single-precision%29))
  (Class|ChaosVehicleMovementComponent|SetThrottleInput (Variables|Default|GetVehicleMovementComponent) AxisValue))

(event Input|AxisEvents|InputAxisBrake
  (params (AxisValue :type Float%20%28single-precision%29))
  (Class|ChaosVehicleMovementComponent|SetBrakeInput (Variables|Default|GetVehicleMovementComponent) AxisValue))

(event Input|AxisEvents|InputAxisSteering
  (params (AxisValue :type Float%20%28single-precision%29))
  (bind _output_get (Variables|Default|SetSteering AxisValue))
  (Class|ChaosVehicleMovementComponent|SetSteeringInput (Variables|Default|GetVehicleMovementComponent) _output_get))

(fn ConstructionScript)