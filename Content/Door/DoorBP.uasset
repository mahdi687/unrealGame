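; Door Blueprint that tells the player character which way the door can open, based on where the player stands.
; Two trigger components, Inwards and Outwards, cast the overlapping actor to PlayerChar and set its OpenInwards or OpenOutwards flag on entry, clearing it on exit.
; The graph contains no door movement; it only writes these flags on the player.
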(event OnComponentBeginOverlap(Inwards)
  (params (OverlappedComponent :type Primitive%20Component%20Object%20Reference) (OtherActor :type Actor%20Object%20Reference) (OtherComp :type Primitive%20Component%20Object%20Reference) (OtherBodyIndex :type Integer) (bFromSweep :type Boolean) (SweepResult :type Hit%20Result%20Structure%20%28by%20ref%29))
  ;[1 1 1] Triggers
  (bind _asplayer_char (Utilities|Casting|CastToPlayerChar OtherActor))
  (Variables|/Game/ThirdPersonDIalogue/Blueprints/PlayerChar.PlayerChar_C|SetOpenInwards _asplayer_char true))

(event OnComponentEndOverlap(Inwards)
  (params (OverlappedComponent :type Primitive%20Component%20Object%20Reference) (OtherActor :type Actor%20Object%20Reference) (OtherComp :type Primitive%20Component%20Object%20Reference) (OtherBodyIndex :type Integer))
  ;[1 1 1] Triggers
  (bind _asplayer_char (Utilities|Casting|CastToPlayerChar OtherActor))
  (Variables|/Game/ThirdPersonDIalogue/Blueprints/PlayerChar.PlayerChar_C|SetOpenInwards _asplayer_char false))

(event OnComponentBeginOverlap(Outwards)
  (params (OverlappedComponent :type Primitive%20Component%20Object%20Reference) (OtherActor :type Actor%20Object%20Reference) (OtherComp :type Primitive%20Component%20Object%20Reference) (OtherBodyIndex :type Integer) (bFromSweep :type Boolean) (SweepResult :type Hit%20Result%20Structure%20%28by%20ref%29))
  ;[1 1 1] Triggers
  (bind _asplayer_char (Utilities|Casting|CastToPlayerChar OtherActor))
  (Variables|/Game/ThirdPersonDIalogue/Blueprints/PlayerChar.PlayerChar_C|SetOpenOutwards _asplayer_char true))

(event OnComponentEndOverlap(Outwards)
  (params (OverlappedComponent :type Primitive%20Component%20Object%20Reference) (OtherActor :type Actor%20Object%20Reference) (OtherComp :type Primitive%20Component%20Object%20Reference) (OtherBodyIndex :type Integer))
  ;[1 1 1] Triggers
  (bind _asplayer_char (Utilities|Casting|CastToPlayerChar OtherActor))
  (Variables|/Game/ThirdPersonDIalogue/Blueprints/PlayerChar.PlayerChar_C|SetOpenOutwards _asplayer_char false))

(fn ConstructionScript)