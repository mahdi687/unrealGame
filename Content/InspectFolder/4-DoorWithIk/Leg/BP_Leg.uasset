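; BP_Leg is a procedural leg that computes a stepping foot position for IK-style placement.
; UpdateFoot finds a target with a forward trace, falling back to a downward trace from the ray's end, then the previous target.
; A planted foot drifting too far flags WantToReplant, while a separate DoReplant flag starts the step.
; Steps interpolate toward the live target using timing and height curves, with optional debug drawing.
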(event Custom|SetDefaultPosition
  (bind _traceposition (Variables|Default|GetTracePosition))
  (CallFunction|GetFootTargetLocation)
  (Variables|Internal|SetPlantStartPosition _traceposition)
  (Variables|Internal|SetTargetPosition _traceposition)
  (Variables|Default|SetFootPosition _traceposition)
  (Variables|Default|SetIsPlanted false))

(event EventBeginPlay
  (Variables|Default|SetFootPosition (Transformation|GetWorldLocation))
  (bind _asbp_third_person_character (Utilities|Casting|CastToBP_ThirdPersonCharacter (Game|GetPlayerCharacter 0)))
  (Variables|Default|SetAnimInstance (Components|SkeletalMesh|GetAnimInstance (Variables|/Script/Engine.Character|GetMesh _asbp_third_person_character))))

(event EventTick
  (params (DeltaSeconds :type Float%20%28single-precision%29)))

(fn UpdateFoot
  (CallFunction|GetFootTargetLocation)
  (CallFunction|CheckforReplant)
  (CallFunction|TakeFootStep)
  (if (Variables|Default|GetDebugDraw)
    (CallFunction|Debug)))

(fn GetFootTargetLocation
  (Utilities|FlowControl|Sequence
    (:then_0
      (Variables|Default|SetRayStart (Transformation|GetWorldLocation)))
    (:then_1
      (Variables|Default|SetRayEnd (+ (Variables|Default|GetRayStart) (* (Math|Vector|GetForwardVector (.Rotation (Math|Transform|BreakTransform (Transformation|GetWorldTransform)))) (Variables|Default|GetRayCastLengh)))))
    (:then_2
      (bind _location (Utilities|CastRay (Variables|Default|GetRayStart) (Variables|Default|GetRayEnd))
        (:True
          (Variables|Default|SetTracePosition _location))
        (:False
          (bind _location_2 (Utilities|CastRay (Variables|Default|GetRayEnd) (- (Variables|Default|GetRayEnd) (Math|Vector|MakeVector 0.0 0.0 (* (Variables|Default|GetRayCastLengh) 4.0))))
            (:True
              (Variables|Default|SetTracePosition _location_2))
            (:False
              (Variables|Default|SetTracePosition (Variables|Internal|GetTargetPosition)))))))
    (:then_3
      (Variables|Internal|SetTargetPosition (Variables|Default|GetTracePosition)))))

(fn CheckforReplant
  (Utilities|FlowControl|Sequence
    (:then_0
      (Variables|Default|SetWantToReplant (and (Variables|Default|GetIsPlanted) (> (Math|Vector|VectorLength (- (Variables|Default|GetFootPosition) (Variables|Internal|GetTargetPosition))) (Variables|Default|GetStopDistance)))))
    (:then_2
      (if (Variables|Default|GetDo%20Replant)
        (Utilities|FlowControl|Sequence
          (:then_0
            (Variables|Default|SetIsPlanted false))
          (:then_1
            (Variables|Internal|SetPlantStartPosition (Variables|Default|GetFootPosition)))
          (:then_2
            (Variables|Internal|SetTimeSinceUnplanted 0.0)))))))

(fn TakeFootStep
  (if (not (Variables|Default|GetIsPlanted))
    (Utilities|FlowControl|Sequence
      (:then_0
        (Variables|Default|SetPrecentageReplanted (/ (Variables|Internal|GetTimeSinceUnplanted) (Variables|Default|GetStopTime))))
      (:then_1
        (Variables|Internal|SetFootPositionNoHeight (Math|Vector|Lerp(Vector) (Variables|Internal|GetPlantStartPosition) (Variables|Internal|GetTargetPosition) (Math|Curves|GetFloatValue (Variables|Default|GetReplantSpeedCurve) (Variables|Default|GetPrecentageReplanted)))))
      (:then_2
        (Variables|Default|SetFootPosition (+ (Variables|Internal|GetFootPositionNoHeight) (Math|Vector|MakeVector 0.0 0.0 (* (Math|Curves|GetFloatValue (Variables|Default|GetReplantCurveHeight) (Variables|Default|GetPrecentageReplanted)) (Variables|Default|GetStopHeight))))))
      (:then_3
        (Variables|Internal|SetTimeSinceUnplanted (+ (Variables|Internal|GetTimeSinceUnplanted) (Utilities|Time|GetWorldDeltaSeconds)))
        (Variables|Default|SetIsPlanted (>= (Variables|Internal|GetTimeSinceUnplanted) (Variables|Default|GetStopTime)))))))

(fn Debug
  (Rendering|Debug|DrawDebugSphere (Variables|Default|GetFootPosition) 4.0 12 "(R=1.000000,G=1.000000,B=1.000000,A=1.000000)" 0.0 2.0))