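; Leg manager component on the third person character that coordinates its left and right leg components for foot placement.
; On BeginPlay it collects both legs from the owning character, then updates each leg's foot every tick.
; CanLegUnplant permits a leg to lift only if another leg is planted.
; GetLegReference resolves a left or right leg tag to the matching component.
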(event Custom|UpdateAllLegs
  (for _array_element (Variables|Default|GetLegs)
    (Default|UpdateFoot _array_element)))

(event EventBeginPlay
  (CallFunction|GetComponentReference))

(event EventTick
  (params (DeltaSeconds :type Float%20%28single-precision%29))
  (CallFunction|UpdateAllLegs))

(fn CanLegUnplant
  (params (Leg :type BP%20Leg%20Object%20Reference))
  (for _array_element (Variables|Default|GetLegs)
    (if (and (Variables|/Game/InspectFolder/4-DoorWithIk/Leg/BP_Leg.BP_Leg_C|GetIsPlanted _array_element) (!= _array_element Leg))
      (return true)))
  (return false))

(fn GetLegReference
  (params (LegTag :type String))
  (bind _asbp_third_person_character (Utilities|Casting|CastToBP_ThirdPersonCharacter (Components|GetOwner)))
  (switch string LegTag
    (:LeftLeg
      (return (Variables|/Game/InspectFolder/Blueprints/BP_ThirdPersonCharacter.BP_ThirdPersonCharacter_C|GetBP_LegLeft _asbp_third_person_character)))
    (:RightLeg
      (return (Variables|/Game/InspectFolder/Blueprints/BP_ThirdPersonCharacter.BP_ThirdPersonCharacter_C|GetBP_LegRight _asbp_third_person_character)))))

(fn GetComponentReference
  (bind _asbp_third_person_character (Utilities|Casting|CastToBP_ThirdPersonCharacter (Components|GetOwner)))
  (Utilities|Array|Add (Variables|Default|GetLegs) (Variables|/Game/InspectFolder/Blueprints/BP_ThirdPersonCharacter.BP_ThirdPersonCharacter_C|GetBP_LegLeft _asbp_third_person_character))
  (Utilities|Array|Add (Variables|Default|GetLegs) (Variables|/Game/InspectFolder/Blueprints/BP_ThirdPersonCharacter.BP_ThirdPersonCharacter_C|GetBP_LegRight _asbp_third_person_character))
  (return))