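; Interactable swinging door that registers itself with the player character when they stand in its trigger box, including an overlap check shortly after BeginPlay.
; Box overlaps pass the door to the character through SetNewDoorMessage and clear it on exit.
; Exposed events play two timelines that yaw DoorRoot for in and out rotation, toggle mesh and handle collision, and store a RightHand reference.
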(event OnComponentBeginOverlap(Box)
  (params (OverlappedComponent :type Primitive%20Component%20Object%20Reference) (OtherActor :type Actor%20Object%20Reference) (OtherComp :type Primitive%20Component%20Object%20Reference) (OtherBodyIndex :type Integer) (bFromSweep :type Boolean) (SweepResult :type Hit%20Result%20Structure%20%28by%20ref%29))
  (if (== OtherActor (Game|GetPlayerCharacter 0))
    (Class|BPIDoor|SetNewDoor(Message) OtherActor self)))

(event OnComponentEndOverlap(Box)
  (params (OverlappedComponent :type Primitive%20Component%20Object%20Reference) (OtherActor :type Actor%20Object%20Reference) (OtherComp :type Primitive%20Component%20Object%20Reference) (OtherBodyIndex :type Integer))
  (Class|BPIDoor|SetNewDoor(Message) OtherActor))

(event Custom|IsOverlapDoor
  (for _array_element (Collision|GetOverlappingActors (Variables|Default|GetBox) 0 :!class /Script/Engine.PrimitiveComponent)
    (if (== _array_element (Game|GetPlayerCharacter 0))
      (Class|BPIDoor|SetNewDoor(Message) _array_element self))))

(event Custom|AttatchRightMouse
  (params (RightHand :type Boolean))
  (Variables|Default|SetRight%20Hand RightHand))

(event Custom|SetCollisionDoor
  (params (Collision :type Boolean))
  (if Collision
    (Collision|SetCollisionEnabled (Variables|Default|GetDoorMesh) "QueryAndPhysics")
    (else
      (Collision|SetCollisionEnabled (Variables|Default|GetDoorMesh) "NoCollision"))))

(event Custom|RotateDoorIn
  (bind _zrotation (Timeline|DoorRotateIn PlayFromStart)
    (:Update
      (Transformation|SetRelativeRotation (Variables|Default|GetDoorRoot) (Math|Rotator|MakeRotator 0.0 0.0 (* _zrotation -9e+01)) false false))))

(event Custom|RotateDoorOut
  (bind _rotationz (Timeline|DoorRotationOut PlayFromStart)
    (:Update
      (Transformation|SetRelativeRotation (Variables|Default|GetDoorRoot) (Math|Rotator|MakeRotator 0.0 0.0 (* _rotationz -9e+01)) false false))))

(event EventBeginPlay
  (bind _asbp_third_person_character (Utilities|Casting|CastToBP_ThirdPersonCharacter (Game|GetPlayerCharacter 0)))
  (Variables|Default|SetPlayer _asbp_third_person_character)
  (Utilities|FlowControl|Delay 0.2)
  (CallFunction|IsOverlapDoor))

(fn ConstructionScript)